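; BP_Chest is a chest that opens once when its box trigger is overlapped and the player's BP_XRPawn has a key.
; BeginPlay creates a Level Sequence player for the opening animation.
; Opening spawns a BP_Note at the Scene component, plays that sequence and calls Begin on every BP_Button in the level.
; Without a key, the pawn shows the WB_NeedKey UI instead.
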(event OnComponentBeginOverlap(Box)
  (params (OverlappedComponent :type Primitive%20Component%20Object%20Reference) (OtherActor :type Actor%20Object%20Reference) (OtherComp :type Primitive%20Component%20Object%20Reference) (OtherBodyIndex :type Integer) (bFromSweep :type Boolean) (SweepResult :type Hit%20Result%20Structure%20%28by%20ref%29))
  (bind _asbp_xrpawn (Utilities|Casting|CastToBP_XRPawn (Game|Player|GetPlayerPawn 0)))
  (if (Variables|/Game/XRFramework/Blueprints/BP_XRPawn.BP_XRPawn_C|GetHasKey _asbp_xrpawn)
    (if (not (Variables|Default|Getchestopened))
      (Variables|Default|Setchestopened true)
      (CallFunction|OpenChest))
    (else
      (bind _asbp_xrpawn_2 (Utilities|Casting|CastToBP_XRPawn (Game|Player|GetPlayerPawn 0)))
      (Default|ShowUI _asbp_xrpawn_2 "WB_NeedKey")
      (Utilities|FlowControl|Delay 3.0))))

(event Custom|OpenChest
  (Game|SpawnActorfromClass "/Game/XRFramework/Blueprints/BP_Note.BP_Note_C" (Transformation|GetWorldTransform (Variables|Default|GetScene)) "AlwaysSpawn" "MultiplyWithRoot" 0 0)
  (Sequencer|Player|Play (Variables|/Script/LevelSequence.LevelSequenceActor|GetSequencePlayer (Variables|Default|GetSeqPlayer)) :!class /Script/MovieScene.MovieSceneSequencePlayer)
  (bind _outactors (Actor|GetAllActorsOfClass "/Game/Puzzle/BP_Button.BP_Button_C"))
  (for _array_element _outactors
    (Default|Begin _array_element)))

(event EventBeginPlay
  (bind _outactor (Sequencer|Player|CreateLevelSequencePlayer (Variables|Default|GetOpenChestSeq)))
  (Variables|Default|SetSeqPlayer _outactor))

(fn ConstructionScript)