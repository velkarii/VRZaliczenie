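; BP_Brain is a puzzle manager that checks whether every BP_Button in the level is switched on.
; Its OnOff event waits briefly, then gathers all BP_Button actors and recounts those with IsOn set.
; When the active count matches the total, it only prints "Otwarte" (Polish for "Open").
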(event EventOnOff
  (Utilities|FlowControl|Delay 0.1)
  (bind _outactors (Actor|GetAllActorsOfClass "/Game/Puzzle/BP_Button.BP_Button_C"))
  (Variables|Default|SetButtonCount (Utilities|Array|Length _outactors))
  (Variables|Default|SetButtonsActive 0)
  (for _array_element _outactors
    (if (Variables|/Game/Puzzle/BP_Button.BP_Button_C|GetisOn? _array_element)
      (Math|Integer|IncrementInt (Variables|Default|GetButtonsActive)
        (:%20%20
          (if (== (Variables|Default|GetButtonsActive) (Variables|Default|GetButtonCount))
            (Development|PrintString "Otwarte")))))))

(fn ConstructionScript)