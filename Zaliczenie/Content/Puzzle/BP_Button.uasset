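; BP_Button is one cell of a Lights Out style puzzle, showing its IsOn state through on and off materials.
; An overlap on the Button component toggles it and calls OnOff on its left, down, up and right neighbor references.
; Each toggle notifies Brain through OnOffMessage.
; A DoOnce reset after a short delay debounces repeated overlaps.
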(event OnComponentBeginOverlap(Button)
  (params (OverlappedComponent :type Primitive%20Component%20Object%20Reference) (OtherActor :type Actor%20Object%20Reference) (OtherComp :type Primitive%20Component%20Object%20Reference) (OtherBodyIndex :type Integer) (bFromSweep :type Boolean) (SweepResult :type Hit%20Result%20Structure%20%28by%20ref%29))
  (Utilities|FlowControl|DoOnce false :!label _label
    (:Completed
      (Default|OnOff (Variables|Default|GetButton_Left))
      (Default|OnOff (Variables|Default|GetButton_Down))
      (Default|OnOff (Variables|Default|GetButton_Up))
      (Default|OnOff (Variables|Default|GetButton_Right))
      (bind _output_get (Variables|Default|SetisOn? (not (Variables|Default|GetisOn?))))
      (if _output_get
        (Rendering|Material|SetMaterial (Variables|Default|GetButton) 0 "/Game/Puzzle/MT_Button_On.MT_Button_On")
        (else
          (Rendering|Material|SetMaterial (Variables|Default|GetButton) 0 "/Game/Puzzle/MT_Button_Off.MT_Button_Off")))
      (Class|BIPuzzle|OnOff(Message) (Variables|Default|GetBrain))
      (Utilities|FlowControl|Delay 0.2)
      (goto _label Reset))))

(event EventBeginPlay
  (if (Variables|Default|GetisOn?)
    (Rendering|Material|SetMaterial (Variables|Default|GetButton) 0 "/Game/Puzzle/MT_Button_On.MT_Button_On")
    (else
      (Rendering|Material|SetMaterial (Variables|Default|GetButton) 0 "/Game/Puzzle/MT_Button_Off.MT_Button_Off"))))

(event EventOnOff
  (bind _output_get (Variables|Default|SetisOn? (not (Variables|Default|GetisOn?))))
  (if _output_get
    (Rendering|Material|SetMaterial (Variables|Default|GetButton) 0 "/Game/Puzzle/MT_Button_On.MT_Button_On")
    (else
      (Rendering|Material|SetMaterial (Variables|Default|GetButton) 0 "/Game/Puzzle/MT_Button_Off.MT_Button_Off")))
  (Class|BIPuzzle|OnOff(Message) (Variables|Default|GetBrain)))

(fn ConstructionScript)